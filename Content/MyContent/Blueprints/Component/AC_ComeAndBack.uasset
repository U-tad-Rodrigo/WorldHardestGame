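; An actor component that moves its owner back and forth along a local direction.
; Tick offsets the owner each frame by Speed times Direction, scaled by delta time and without sweeping.
; A looping timer started at BeginPlay negates Speed every Time seconds to reverse the motion.
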(event `self.ReceiveBeginPlay`
  (`KismetSystemLibrary.K2_SetTimerDelegate` (delegate `OnTimerEnds`) (`self.Time`) true))

(event `OnTimerEnds`
  (set `self.speed` (* (`self.speed`) -1.0)))

(event `self.ReceiveTick`
  (params (DeltaSeconds :type "Float (single-precision)"))
  (`Actor.K2_AddActorLocalOffset` (`self.GetOwner`) (* DeltaSeconds (`self.speed`) (`self.direction`)) false false))