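; Actor component that moves its owner in a horizontal circle, apparently intended for a ball, periodically reversing direction.
; BeginPlay stores the owner's location as the center, converts the start angle offset to radians and starts a looping timer that negates Speed.
; Tick advances the angle by Speed, wraps it at 2π, and sets the owner's position from cosine and sine scaled by Radius, without sweeping.
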(event `self.ReceiveTick`
  (params (DeltaSeconds :type "Float (single-precision)"))
  ; Calcular la velocidad final de la bola, al final se pasa a Vector
  (bind _output_get (set `self.Angle` (`KismetMathLibrary.FMod` (+ (* DeltaSeconds (`self.Speed`)) (`self.Angle`)) (* (`KismetMathLibrary.GetPI`) 2.0))))
  (`self.AngleToVector` _output_get _output_get))

(event `self.ReceiveBeginPlay`
  (set `self.Center` (`Actor.K2_GetActorLocation` (`self.GetOwner`)))
  (`self.StartAngleToRadian`)
  (`KismetSystemLibrary.K2_SetTimerDelegate` (delegate `OnTimerEnds`) (`self.Seconds`) true))

(event `OnTimerEnds`
  (set `self.speed` (* (`self.speed`) -1.0)))

(fn `AngleToVector`
  (params (A :type "Float (double-precision)") (A2 :type "Float (double-precision)"))
  (`Actor.K2_SetActorLocation` (`self.GetOwner`) (+ (`KismetMathLibrary.MakeVector` (* (`self.Radius`) (`KismetMathLibrary.Cos` A2)) (* (`KismetMathLibrary.Sin` A) (`self.Radius`))) (`self.Center`)) false false))

(fn `StartAngleToRadian`
  (set `self.Angle` (/ (* (`self.StartAngleOffset`) (`KismetMathLibrary.GetPI`)) 180.0)))