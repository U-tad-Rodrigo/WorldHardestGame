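; Player pawn: a physics cube that collects coins, uses teleporters and checkpoints, and opens the Final level at the goal.
; Movement applies a camera-yaw-relative force at the cube's top, so it tips and rolls.
; Overlaps branch on actor tags; any untagged actor, such as a ball, respawns it at the last checkpoint or PlayerStart.
; BP_MyPlayerController tallies coins and deaths, and the teleport target switches to TPLocation2 after first use.
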(event `EnhancedInput|/Game/MyContent/Blueprints/Inputs/IA_Move`
  (params (ActionValue :type "Vector2D Structure") (ElapsedSeconds :type "Float (double-precision)") (TriggeredSeconds :type "Float (double-precision)") (InputAction :type "InputAction Object Reference" :default "/Game/MyContent/Blueprints/Inputs/IA_Move.IA_Move"))
  (:`Triggered`
    (bind _returnvalue (`self.VectorToForce` ActionValue))
    (bind _returnvalue_2 (`self.GetForcePivot`))
    (`PrimitiveComponent.AddForceAtLocation` (`self.Cube`) _returnvalue _returnvalue_2 "None")))

(event `self.ReceiveTick`
  (params (DeltaSeconds :type "Float (single-precision)")))

(event `self.ReceiveActorBeginOverlap`
  (params (OtherActor :type "Actor Object Reference"))
  ; cadena de chains, para verificar si es Moneda, Checkpoint, Teletransportador o Bola (else)
  (if (`self.ActorHasTag` OtherActor "Coin")
    (`self.OnCoin` OtherActor)
    (elif (`self.ActorHasTag` OtherActor "TP")
      (`self.K2_SetActorLocation` (`self.TPLocation`))
      (set `self.TPLocation` (`self.TPLocation2`))
      (elif (`self.ActorHasTag` OtherActor "Checkpoint")
        (set `self.InitLocation` (`self.K2_GetActorLocation` OtherActor))
        (elif (`self.ActorHasTag` OtherActor "FINAL")
          (`GameplayStatics.OpenLevelBySoftObjectPtr` "/Game/MyContent/Levels/Final.Final")
          (else
            (`self.K2_SetActorLocation` (`self.InitLocation`))
            (`self.OnDeath`)))))))

(event `self.ReceiveBeginPlay`
  (bind _returnvalue (`GameplayStatics.GetActorOfClass` "/Script/Engine.PlayerStart"))
  (set `self.InitLocation` (`self.K2_GetActorLocation` _returnvalue))
  ; cadena de chains, para verificar si es Moneda, Checkpoint, Teletransportador o Bola (else)
  (set `self.HalfSize` (.z (`.BoxExtent` (`KismetSystemLibrary.GetComponentBounds` (`self.Cube`))))) ; half Size se usa para aplicar la fuerza en la parte de arriba del cubo
)

(fn `GetForcePivot`
  (returns (ReturnValue :type "Vector Structure"))
  (return (+ (`self.K2_GetActorLocation`) (`KismetMathLibrary.MakeVector` 0.0 0.0 (`self.HalfSize`)))))

(fn `OnCoin`
  (params (ActorToDestroy :type "Actor Object Reference"))
  (`self.K2_DestroyActor` ActorToDestroy)
  (bind _asbp_my_player_controller (cast `/Game/MyContent/Blueprints/Framework/BP_MyPlayerController` (`self.GetController`)))
  (`/Game/MyContent/Blueprints/Framework/BP_MyPlayerController.UpdateScore` _asbp_my_player_controller))

(fn `OnDeath`
  (bind _asbp_my_player_controller (cast `/Game/MyContent/Blueprints/Framework/BP_MyPlayerController` (`self.GetController`)))
  (`/Game/MyContent/Blueprints/Framework/BP_MyPlayerController.Update Death` _asbp_my_player_controller))

(fn `UserConstructionScript`)

(fn `VectorToForce`
  (params (InVec :type "Vector2D Structure"))
  (returns (ReturnValue :type "Vector Structure"))
  (bind (_x _y) (`KismetMathLibrary.BreakVector2D` InVec))
  (bind _returnvalue (`KismetMathLibrary.MakeRotator` 0.0 0.0 (.yaw (`self.GetControlRotation`))))
  (return (* (`KismetMathLibrary.Normal` (+ (* _x (`KismetMathLibrary.GetForwardVector` _returnvalue)) (* _y (`KismetMathLibrary.GetRightVector` _returnvalue)))) (`self.Speed`))))