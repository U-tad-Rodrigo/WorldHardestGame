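; Player controller that handles camera input and tracks the player's score and deaths.
; On BeginPlay it hides the cursor, adds the Enhanced Input mapping context and creates the main HUD widget.
; Camera input turns the control rotation with clamped pitch, and zoom adjusts the pawn's spring arm length within limits.
; Score and death updates increment counters, refresh the widget text and copy the values to BP_GameInstance.
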(event `self.ReceiveBeginPlay`
  (set `self.bShowMouseCursor` false)
  (`self.InitInputs`)
  (bind _returnvalue (`|CreateWidget` "/Game/MyContent/Blueprints/UI/WBP_MainWidget.WBP_MainWidget_C"))
  (bind _output_get (set `self.MyWidget` _returnvalue))
  (`UserWidget.AddToViewport` _output_get 0))

(event `EnhancedInput|/Game/MyContent/Blueprints/Inputs/IA_Camera`
  (params (ActionValue :type "Vector2D Structure") (ElapsedSeconds :type "Float (double-precision)") (TriggeredSeconds :type "Float (double-precision)") (InputAction :type "InputAction Object Reference" :default "/Game/MyContent/Blueprints/Inputs/IA_Camera.IA_Camera"))
  (:`Triggered`
    (bind _returnvalue (`self.CameraRotation` ActionValue))
    (`self.SetControlRotation` _returnvalue)))

(event `EnhancedInput|/Game/MyContent/Blueprints/Inputs/IA_Zoom`
  (params (ActionValue :type "Float (double-precision)") (ElapsedSeconds :type "Float (double-precision)") (TriggeredSeconds :type "Float (double-precision)") (InputAction :type "InputAction Object Reference" :default "/Game/MyContent/Blueprints/Inputs/IA_Zoom.IA_Zoom"))
  (:`Triggered`
    (bind (_returnvalue _returnvalue2) (`self.SetCameraZoom` ActionValue))
    (set `SpringArmComponent.TargetArmLength` _returnvalue _returnvalue2)))

(fn `CameraRotation`
  (params (InVec :type "Vector2D Structure"))
  (returns (ReturnValue :type "Rotator Structure"))
  (bind (_x _y) (`KismetMathLibrary.BreakVector2D` InVec))
  (return (`KismetMathLibrary.MakeRotator` 0.0 (`KismetMathLibrary.FClamp` (+ (.pitch (`self.GetControlRotation`)) (* (`self.SensPitch`) _y)) -70.0 -15.0) (+ (.yaw (`self.GetControlRotation`)) (* _x (`self.SensYaw`))))))

(fn `InitInputs`
  (`EnhancedInputSubsystemInterface.AddMappingContext` (subsystem `EnhancedInputLocalPlayerSubsystem`) "/Game/MyContent/Blueprints/Inputs/MappingContext.MappingContext" 0 (struct)))

(fn `SetCameraZoom`
  (params (A :type "Float (double-precision)"))
  (returns (ReturnValue :type "Float (double-precision)") (ReturnValue2 :type "SpringArmComponent Object Reference"))
  (bind _returnvalue (`self.GetComponentByClass` (`self.K2_GetPawn`) "/Script/Engine.SpringArmComponent"))
  (return (`KismetMathLibrary.FClamp` (+ (* A (`self.ZoomSpeed`)) (`SpringArmComponent.TargetArmLength` _returnvalue)) 300.0 900.0) _returnvalue))

(fn `Update Death`
  (bind _output_get (set `self.Deaths` (+ (`self.Deaths`) 1)))
  (`TextBlock.SetText` (`/Game/MyContent/Blueprints/UI/WBP_MainWidget.Deaths` (`self.MyWidget`)) (`KismetTextLibrary.Conv_StringToText` (`KismetStringLibrary.Concat_StrStr` "Deaths: " (`KismetStringLibrary.Conv_IntToString` _output_get))))
  (bind _asbp_game_instance (cast `/Game/MyContent/Blueprints/BP_GameInstance` (`GameplayStatics.GetGameInstance`)))
  (set `/Game/MyContent/Blueprints/BP_GameInstance.Deaths` (`self.Deaths`) _asbp_game_instance))

(fn `UpdateScore`
  (bind _output_get (set `self.Score` (+ (`self.Score`) 1)))
  (`TextBlock.SetText` (`/Game/MyContent/Blueprints/UI/WBP_MainWidget.ScoreText` (`self.MyWidget`)) (`KismetTextLibrary.Conv_StringToText` (`KismetStringLibrary.Concat_StrStr` "Score: " (`KismetStringLibrary.Conv_IntToString` _output_get))))
  (bind _asbp_game_instance (cast `/Game/MyContent/Blueprints/BP_GameInstance` (`GameplayStatics.GetGameInstance`)))
  (set `/Game/MyContent/Blueprints/BP_GameInstance.Score` (`self.Score`) _asbp_game_instance))

(fn `UserConstructionScript`)